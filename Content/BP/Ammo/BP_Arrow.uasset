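; Arrow projectile actor driven by a state machine (in hand, in air, in enemy body, in object) that sets collision and projectile movement.
; Shooting adds a projectile component; enemy overlaps trigger a forward trace, notify the enemy, and grab the hit bone with a physics handle.
; The handle follows the arrow, dragging the body until the arrow hits a CanArrowIn-tagged object, where it stops.
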(event `self.ReceiveBeginPlay`
  (`self.StateChange` "NewEnumerator0"))

(event `ShotArrow`
  (params (ShotDir :type "Vector Structure"))
  (set `self.Shot Dir` ShotDir)
  (`self.StateChange` "NewEnumerator1"))

(event `self.StopCollision.OnComponentBeginOverlap`
  (params (OverlappedComponent :type "PrimitiveComponent Object Reference") (OtherActor :type "Actor Object Reference") (OtherComp :type "PrimitiveComponent Object Reference") (OtherBodyIndex :type Integer) (bFromSweep :type Boolean) (SweepResult :type "HitResult Structure (by ref)"))
  (bind _returnvalue (`self.K2_GetActorLocation`))
  (`|ExecutionSequence`
    (:`then_0`
      (bind _asbp_enemy (cast `/Game/ThirdPersonBP/Blueprints/BP_Enemy` OtherActor))
      (set `self.HitEnemy` _asbp_enemy)
      (`self.StateChange` "NewEnumerator2")
      (bind (_outhit _returnvalue_2) (`KismetSystemLibrary.LineTraceSingle` :`Start` _returnvalue :`End` (+ _returnvalue (* (`KismetMathLibrary.Normal` (- (`SceneComponent.K2_GetComponentLocation` (`self.ArrowHead`)) _returnvalue)) 1000.0)) :`TraceChannel` "TraceTypeQuery1" :`bTraceComplex` true :`DrawDebugType` "Persistent"))
      (if _returnvalue_2
        (`/Game/ThirdPersonBP/Blueprints/BP_Enemy.BPI_GetHitByArrow` (`self.HitEnemy`) (`MovementComponent.Velocity` (`self.ProjectileComponent`)))
        (bind (_bblockinghit _binitialoverlap _time _distance _location _impactpoint _normal _impactnormal _physmat _hitactor _hitcomponent _hitbonename) (`GameplayStatics.BreakHitResult` _outhit))
        (cast `/Game/ThirdPersonBP/Blueprints/BP_Enemy` _hitactor)
        (bind _returnvalue_3 (`AddComponent|NODE_AddPhysicsHandleComponent-0`))
        (bind _output_get (set `self.PhysicsHandle` _returnvalue_3))
        (`PhysicsHandleComponent.GrabComponentAtLocation` _output_get (`Character.Mesh` (`self.HitEnemy`)) _hitbonename _location)))
    (:`then_1`
      (if (`self.ActorHasTag` OtherActor "CanArrowIn")
        (`self.StateChange` "NewEnumerator3")))))

(event `self.ReceiveTick`
  (params (DeltaSeconds :type "Float (single-precision)"))
  (`/Engine/EditorBlueprintResources/StandardMacros.IsValid` (`self.PhysicsHandle`)
    (:`Is Valid`
      (if (not (`|EnumEquality` (`self.ArrowState`) "NewEnumerator3"))
        (`self.UpdateGrabLocation`)))))

(event `UpdateGrabLocation`
  (`PhysicsHandleComponent.SetTargetLocation` (`self.PhysicsHandle`) (`SceneComponent.K2_GetComponentLocation` (`self.StopCollision`))))

(fn `StateChange`
  (params (StateToChange :type "/Game/BP/Ammo/ENUM_ArrowState Enum" :default "NewEnumerator0"))
  (bind _stopcollision (`self.StopCollision`))
  (set `self.ArrowState` StateToChange)
  (switch `/Game/BP/Ammo/ENUM_ArrowState` StateToChange
    (:`NewEnumerator0`
      (`PrimitiveComponent.SetCollisionEnabled` (`self.Sphere Collision`) "NoCollision")
      (`PrimitiveComponent.SetCollisionEnabled` _stopcollision "NoCollision"))
    (:`NewEnumerator1`
      (`PrimitiveComponent.SetCollisionEnabled` (`self.Sphere Collision`) "NoCollision")
      (`PrimitiveComponent.SetCollisionEnabled` _stopcollision "QueryOnly")
      (bind _returnvalue (`AddComponent|NODE_AddProjectileMovementComponent-0`))
      (bind _output_get (set `self.ProjectileComponent` _returnvalue))
      (set `MovementComponent.Velocity` (* (`self.Shot Dir`) 5000.0) _output_get)
      (`KismetSystemLibrary.PrintString` "InAir"))
    (:`NewEnumerator2`
      (`PrimitiveComponent.SetCollisionEnabled` (`self.Sphere Collision`) "NoCollision")
      (`PrimitiveComponent.SetCollisionEnabled` _stopcollision "QueryOnly"))
    (:`NewEnumerator3`
      (`PrimitiveComponent.SetCollisionEnabled` (`self.Sphere Collision`) "QueryOnly")
      (`PrimitiveComponent.SetCollisionEnabled` _stopcollision "NoCollision")
      (`MovementComponent.StopMovementImmediately` (`self.ProjectileComponent`))
      (`ActorComponent.K2_DestroyComponent` (`self.ProjectileComponent`)))))

(fn `UserConstructionScript`)