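; BP_Monster is an actor that destroys itself two seconds after BeginPlay and announces its death, apparently demonstrating two Blueprint communication methods.
; The IsInterface flag selects between sending BPIFlyAwayMessage to every BPI_FlyAway implementer and calling the EventDead dispatcher.
; Both paths print debug text naming the method before destroying the actor.
; An unconnected lookup of BP_MonsterBaby actors never runs.
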(event `self.ReceiveBeginPlay`
  (`KismetSystemLibrary.K2_SetTimerDelegate` (delegate `DestroySelf`) 2.0))

(event `DestroySelf`
  (if (`self.IsInterface`)
    (bind _outactors (`GameplayStatics.GetAllActorsWithInterface` "/Game/BPI/BPI_FlyAway.BPI_FlyAway_C"))
    (for _array_element _outactors
      (message `/Game/BPI/BPI_FlyAway.BPI_FlyAway` _array_element)
      (`KismetSystemLibrary.PrintString` "I\\m Dead   -------  call Interface" true true (struct :`R` 0.323959 :`G` 1.0 :`B` 0.365537 :`A` 1.0)))
    (`self.K2_DestroyActor`)
    (else
      (`self.EventDead`)
      (`KismetSystemLibrary.PrintString` "I\\m Dead   -------  call Event Dispatcher")
      (`self.K2_DestroyActor`))))

(fn `UserConstructionScript`)